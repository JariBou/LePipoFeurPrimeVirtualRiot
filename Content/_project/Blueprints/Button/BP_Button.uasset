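; Pressure button that sinks while anything overlaps it and fires OnActivated when pressed down past a height threshold.
; Overlap counters drive Tick, which steps the button between zero and its starting offset via MoveComponentTo.
; A second "coyotee" volume stops the button rising while occupied, acting as a release buffer.
; TryButtonToggle compares height to the threshold each tick; deactivation only resets the flag and prints.
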(event `self.ReceiveBeginPlay`
  ; Setup Button
  (`self.TryButtonToggle`))

(event `self.ButtonCollision.OnComponentBeginOverlap`
  (params (OverlappedComponent :type "PrimitiveComponent Object Reference") (OtherActor :type "Actor Object Reference") (OtherComp :type "PrimitiveComponent Object Reference") (OtherBodyIndex :type Integer) (bFromSweep :type Boolean) (SweepResult :type "HitResult Structure (by ref)"))
  ; Begin Overlap
  (if (not (== OtherActor self))
    (bind _result (`/Engine/EditorBlueprintResources/StandardMacros.IncrementInt` (`self.NbPushers`)))))

(event `self.ReceiveTick`
  (params (DeltaSeconds :type "Float (single-precision)"))
  (bind (_relativelocation_x _relativelocation_y _relativelocation_z) (`KismetMathLibrary.BreakVector` (`SceneComponent.RelativeLocation` (`self.Button`))))
  (bind (_relativelocation_x_2 _relativelocation_y_2 _relativelocation_z_2) (`KismetMathLibrary.BreakVector` (`SceneComponent.RelativeLocation` (`self.Button`))))
  ; Button Tick
  (`|ExecutionSequence`
    (:`then_0`
      (if (> (`self.NbPushers`) 0)
        (set `self.TargetOffset` (`KismetMathLibrary.FClamp` (- _relativelocation_z 5.0) 0.0 (`self.StartButtonOffset`)))
        (`KismetSystemLibrary.MoveComponentTo` (`self.Button`) (`KismetMathLibrary.MakeVector` 0.0 0.0 (`self.TargetOffset`)) (struct) false false 0.1 :!label _label)
        (elif (<= (`self.NbCoyoteePushers`) 0)
          (set `self.TargetOffset` (`KismetMathLibrary.FClamp` (+ _relativelocation_z_2 5.0) 0.0 (`self.StartButtonOffset`)))
          (goto _label))))
    (:`then_1`
      (`self.TryButtonToggle`))))

(event `self.ButtonCollision.OnComponentEndOverlap`
  (params (OverlappedComponent :type "PrimitiveComponent Object Reference") (OtherActor :type "Actor Object Reference") (OtherComp :type "PrimitiveComponent Object Reference") (OtherBodyIndex :type Integer))
  ; End Overlap
  (if (not (== null self))
    (bind _result (`/Engine/EditorBlueprintResources/StandardMacros.DecrementInt` (`self.NbPushers`)))))

(event `self.CoyoteeCollision.OnComponentBeginOverlap`
  (params (OverlappedComponent :type "PrimitiveComponent Object Reference") (OtherActor :type "Actor Object Reference") (OtherComp :type "PrimitiveComponent Object Reference") (OtherBodyIndex :type Integer) (bFromSweep :type Boolean) (SweepResult :type "HitResult Structure (by ref)"))
  ; Coyotee Overlap
  (if (not (== null self))
    (`/Engine/EditorBlueprintResources/StandardMacros.IncrementInt` (`self.NbCoyoteePushers`))))

(event `self.CoyoteeCollision.OnComponentEndOverlap`
  (params (OverlappedComponent :type "PrimitiveComponent Object Reference") (OtherActor :type "Actor Object Reference") (OtherComp :type "PrimitiveComponent Object Reference") (OtherBodyIndex :type Integer))
  ; Coyotee Overlap
  (if (not (== null self))
    (`/Engine/EditorBlueprintResources/StandardMacros.DecrementInt` (`self.NbCoyoteePushers`))))

(fn `TryButtonToggle`
  (bind (_relativelocation_x _relativelocation_y _relativelocation_z) (`KismetMathLibrary.BreakVector` (`SceneComponent.RelativeLocation` (`self.Button`))))
  (bind (_relativelocation_x_2 _relativelocation_y_2 _relativelocation_z_2) (`KismetMathLibrary.BreakVector` (`SceneComponent.RelativeLocation` (`self.Button`))))
  (if (`self.bActivated`)
    (if (> _relativelocation_z (`self.ActivationOffsetThreshold`))
      (set `self.bActivated` false)
      (`KismetSystemLibrary.PrintString` "Deactivate Button" true true (struct :`R` 0.429856 :`G` 0.313735 :`B` 1.0 :`A` 1.0)))
    (elif (<= _relativelocation_z_2 (`self.ActivationOffsetThreshold`))
      (set `self.bActivated` true)
      (`KismetSystemLibrary.PrintString` "Activate Button" true true (struct :`R` 0.429856 :`G` 0.313735 :`B` 1.0 :`A` 1.0))
      (`self.OnActivated`))))

(fn `UserConstructionScript`
  (`SceneComponent.K2_SetRelativeLocation` (`self.Button`) (`KismetMathLibrary.MakeVector` 0.0 0.0 (`self.StartButtonOffset`)) false false))