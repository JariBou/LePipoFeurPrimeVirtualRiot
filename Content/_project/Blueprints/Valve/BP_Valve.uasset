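; BP_Valve is a grabbable valve that a player turns about its yaw axis with a motion controller.
; BP_GrabComponent events record the grabbing controller on grab and clear it on drop.
; While grabbed, Tick finds the controller's angle in the valve's local XY plane with Atan2.
; It adds that angle, scaled by delta time and RotationSpeed, to yaw, so local X eases toward the hand.
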(event `self.ReceiveTick`
  (params (DeltaSeconds :type "Float (single-precision)"))
  (if (`self.IsGrabbed`)
    (`self.RotateValve` (`self.GrabbingMotionController`) DeltaSeconds)))

(event `self.BP_GrabComponent.OnGrabbed`
  (params (MotionController :type "MotionControllerComponent Object Reference") (ActorGrabbed :type "Actor Object Reference"))
  (set `self.IsGrabbed` true)
  (set `self.GrabbingMotionController` MotionController))

(event `self.BP_GrabComponent.OnDropped`
  (params (ActorDropped :type "Actor Object Reference"))
  (set `self.IsGrabbed` false)
  (set `self.GrabbingMotionController` null))

(fn `ComputeTargetRotation`
  (params (MotionController :type "MotionControllerComponent Object Reference"))
  (returns (OutRotation :type "Float (double-precision)"))
  (bind (_returnvalue_x _returnvalue_y) (`KismetMathLibrary.BreakVector` (`KismetMathLibrary.InverseTransformLocation` (`self.GetTransform`) (`SceneComponent.K2_GetComponentLocation` MotionController))))
  (`/Engine/EditorBlueprintResources/StandardMacros.IsValid` MotionController
    (:`Is Valid`
      (return (`KismetMathLibrary.DegAtan2` _returnvalue_y _returnvalue_x)))))

(fn `RotateValve`
  (params (MotionController :type "MotionControllerComponent Object Reference") (DeltaTime :type "Float (double-precision)"))
  (bind (_returnvalue_roll _returnvalue_pitch _returnvalue_yaw) (`KismetMathLibrary.BreakRotator` (`self.K2_GetActorRotation`)))
  (bind _outrotation (`self.ComputeTargetRotation` MotionController))
  (`self.K2_SetActorRotation` (`KismetMathLibrary.MakeRotator` _returnvalue_roll _returnvalue_pitch (+ _returnvalue_yaw (* (* (- _outrotation 0.0) DeltaTime) (`self.RotationSpeed`))))))

(fn `UserConstructionScript`)