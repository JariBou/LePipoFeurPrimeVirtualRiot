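; BP_RotatingCube is a grabbable actor whose cube rotates around yaw to follow the motion controller holding it.
; On grab, it stores the controller and the cube's relative rotation, then starts a looping timer calling UpdateRotation instead of using Tick.
; Each update adds the look-at yaw toward the controller to the stored yaw, or releases the grab beyond MaxDistance.
; Dropping clears the timer and controller reference.
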(event `self.BP_GrabComponent.OnGrabbed`
  (params (MotionController :type "MotionControllerComponent Object Reference") (ActorGrabbed :type "Actor Object Reference"))
  (set `self.Motion Controller` MotionController)
  (set `self.Cube Rotation Var` (`SceneComponent.RelativeRotation` (`self.Cube`)))
  (bind _returnvalue (`KismetSystemLibrary.K2_SetTimer` null "UpdateRotation" 0.02 true true))
  (set `self.Timer` _returnvalue))

(event `self.BP_GrabComponent.OnDropped`
  (params (ActorDropped :type "Actor Object Reference"))
  (`KismetSystemLibrary.K2_ClearAndInvalidateTimerHandle` (`self.Timer`))
  (set `self.Motion Controller` null))

(fn `UpdateRotation`
  (bind (_cube_rotation_var_roll _cube_rotation_var_pitch _cube_rotation_var_yaw) (`KismetMathLibrary.BreakRotator` (`self.Cube Rotation Var`)))
  (bind _returnvalue (`SceneComponent.K2_GetComponentLocation` (`self.Cube`)))
  (bind _returnvalue_2 (`SceneComponent.K2_GetComponentLocation` (`self.Motion Controller`)))
  (bind (_returnvalue_roll _returnvalue_pitch _returnvalue_yaw) (`KismetMathLibrary.BreakRotator` (`KismetMathLibrary.FindLookAtRotation` _returnvalue _returnvalue_2)))
  (if (> (`KismetMathLibrary.Vector_Distance` _returnvalue _returnvalue_2) (`self.MaxDistance`))
    (`/Game/_project/Blueprints/BP_GrabComponent.TryRelease` (`self.BP_GrabComponent`))
    (else
      (`SceneComponent.K2_SetRelativeRotation` (`self.Cube`) (`KismetMathLibrary.MakeRotator` _cube_rotation_var_roll _cube_rotation_var_pitch (+ _cube_rotation_var_yaw _returnvalue_yaw)) false false))))

(fn `UserConstructionScript`)