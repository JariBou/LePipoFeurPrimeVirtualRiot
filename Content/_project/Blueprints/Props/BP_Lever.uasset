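; BP_Lever is a VR lever prop that pivots while a motion controller holds its GrabComponent.
; Grabbing stores the controller and starts a fast looping timer on UpdateRotation; dropping clears both.
; Each tick converts the controller transform into GrabComponent space and adds a scaled vertical offset, measured against the component's relative location, to the Scene component's roll.
; Roll is clamped to a fixed range, while pitch and yaw are preserved.
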(event `self.GrabComponent.OnGrabbed`
  (params (`Motion Controller` :type "MotionControllerComponent Object Reference"))
  (set `self.Motion Controller` `Motion Controller`)
  (bind _returnvalue (`KismetSystemLibrary.K2_SetTimer` null "UpdateRotation" 0.01 true true))
  (set `self.Timer` _returnvalue)
  (`KismetSystemLibrary.PrintString` "Grab"))

(event `self.GrabComponent.OnDropped`
  (`KismetSystemLibrary.K2_ClearAndInvalidateTimerHandle` (`self.Timer`))
  (set `self.Motion Controller` null)
  (`KismetSystemLibrary.PrintString` "Drop"))

(fn `UpdateRotation`
  (bind _grabcomponent (`self.GrabComponent`))
  (bind _scene (`self.Scene`))
  (bind (_returnvalue_location _returnvalue_rotation _returnvalue_scale) (`KismetMathLibrary.BreakTransform` (`SceneComponent.K2_GetComponentToWorld` (`self.Motion Controller`))))
  (bind (_returnvalue_location_2 _returnvalue_rotation_2 _returnvalue_scale_2) (`KismetMathLibrary.BreakTransform` (`SceneComponent.K2_GetComponentToWorld` _grabcomponent)))
  (bind (_relativerotation_roll _relativerotation_pitch _relativerotation_yaw) (`KismetMathLibrary.BreakRotator` (`SceneComponent.RelativeRotation` _scene)))
  (bind _returnvalue_location_3 (`KismetMathLibrary.BreakTransform` (`KismetMathLibrary.MakeRelativeTransform` (`KismetMathLibrary.MakeTransform` _returnvalue_location _returnvalue_rotation _returnvalue_scale) (`KismetMathLibrary.MakeTransform` _returnvalue_location_2 _returnvalue_rotation_2 _returnvalue_scale_2))))
  (bind (_returnvalue_x _returnvalue_y _returnvalue_z) (`KismetMathLibrary.BreakVector` (- (`SceneComponent.RelativeLocation` _grabcomponent) _returnvalue_location_3)))
  (`SceneComponent.K2_SetRelativeRotation` _scene (`KismetMathLibrary.MakeRotator` (`KismetMathLibrary.FClamp` (+ _relativerotation_roll (/ _returnvalue_z 10.0)) -90.0 50.0) _relativerotation_pitch _relativerotation_yaw) false false))

(fn `UserConstructionScript`)