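; BP_Brick is a grabbable brick prop that breaks walls of a matching type on impact.
; On BeginPlay it spawns a BP_MasterFieldTest actor at the grab component's transform and attaches it to itself.
; A hit passing the collision channel check against a Wall whose type matches TypeOfWallBreaker triggers that field, then destroys both field and brick.
; Grab and drop events only update the IsGrabed flag, which the hit logic ignores.
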(event `self.ReceiveBeginPlay`
  (bind _returnvalue (`|SpawnActorFromClass` "/Game/_project/Blueprints/BP_MasterFieldTest.BP_MasterFieldTest_C" (`SceneComponent.K2_GetComponentToWorld` (`self.BP_GrabComponent`)) "AlwaysSpawn" "MultiplyWithRoot" self null))
  (bind _output_get (set `self.MasterField` _returnvalue))
  (`self.K2_AttachToActor` _output_get self "None" "KeepWorld" "KeepWorld" "KeepWorld" true))

(event `self.BP_GrabComponent.OnGrabbed`
  (params (MotionController :type "MotionControllerComponent Object Reference") (ActorGrabbed :type "Actor Object Reference"))
  (set `self.IsGrabed` true))

(event `self.BP_GrabComponent.OnDropped`
  (params (ActorDropped :type "Actor Object Reference"))
  (set `self.IsGrabed` false))

(event `self.Brick.OnComponentHit`
  (params (HitComponent :type "PrimitiveComponent Object Reference") (OtherActor :type "Actor Object Reference") (OtherComp :type "PrimitiveComponent Object Reference") (NormalImpulse :type "Vector Structure") (Hit :type "HitResult Structure (by ref)"))
  (bind (_bblockinghit _binitialoverlap _time _distance _location _impactpoint _normal _impactnormal _physmat _hitactor _hitcomponent) (`GameplayStatics.BreakHitResult` Hit))
  (if (`|EnumEquality` (`PrimitiveComponent.GetCollisionObjectType` _hitcomponent) "ECC_GameTraceChannel3")
    (bind _aswall (cast `/Game/_project/Blueprints/Props/Wall` _hitactor)
      (:`then`
        (if (`|EnumEquality` (`/Game/_project/Blueprints/Props/Wall.TypeOfWall` _aswall) (`self.TypeOfWallBreaker`))
          (`/Engine/EditorResources/FieldNodes/FS_MasterField.CE_Trigger` (`self.MasterField`))
          (`self.K2_DestroyActor` (`self.MasterField`))
          (`self.K2_DestroyActor`)))
      (:`CastFailed`
        (`KismetSystemLibrary.PrintText` "Not Real Wall")))))

(fn `UserConstructionScript`)