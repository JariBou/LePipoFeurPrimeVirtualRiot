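; BP_DoorSwingV2 is a VR swinging door that rotates around a Pivot component while grabbed by a motion controller.
; GrabComponent events store the controller on grab and clear it on drop.
; While held, Tick derives yaw from a controller-to-pivot look-at rotation, offset and clamped to a 90-degree swing either way.
; When released, the door snaps shut if nearly at zero world yaw, so limits and closed pose are world-space.
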(event `self.GrabComponent.OnGrabbed`
  (set `self.MotionController` (`/Game/VRTemplate/Blueprints/GrabComponent.MotionControllerRef` (`self.GrabComponent`))))

(event `self.GrabComponent.OnDropped`
  (set `self.MotionController` null))

(event `self.ReceiveTick`
  (params (DeltaSeconds :type "Float (single-precision)"))
  (bind _motioncontroller (`self.MotionController`))
  (bind (_returnvalue_roll _returnvalue_pitch _returnvalue_yaw) (`KismetMathLibrary.BreakRotator` (`SceneComponent.K2_GetComponentRotation` (`self.Pivot`))))
  (bind (_returnvalue_roll_2 _returnvalue_pitch_2 _returnvalue_yaw_2) (`KismetMathLibrary.BreakRotator` (`KismetMathLibrary.FindLookAtRotation` (`SceneComponent.K2_GetComponentLocation` _motioncontroller) (`SceneComponent.K2_GetComponentLocation` (`self.Pivot`)))))
  (`/Engine/EditorBlueprintResources/StandardMacros.IsValid` _motioncontroller
    (:`Is Valid`
      (`SceneComponent.K2_SetWorldRotation` (`self.Pivot`) (`KismetMathLibrary.MakeRotator` 0.0 0.0 (`KismetMathLibrary.ClampAngle` (- _returnvalue_yaw_2 90.0) -90.0 90.0)) false false))
    (:`Is Not Valid`
      (if (`KismetMathLibrary.NearlyEqual_FloatFloat` _returnvalue_yaw 0.0 5.0)
        (`SceneComponent.K2_SetWorldRotation` (`self.Pivot`) (`KismetMathLibrary.MakeRotator` 0.0) false false)))))

(fn `UserConstructionScript`)